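; BP_Enemy is an enemy that turns to face opposite the player camera's yaw every tick and caches the player character's Health at BeginPlay.
; FollowPlayer loops an AI move toward the player, while RunAway moves 500 units away, waits two seconds, then resumes following.
; Both movement events have no live caller here to start them, so only the Wait rotation runs from this graph, with debug prints.
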(event Custom|Follow%20Player
  (Development|PrintString "Follow")
  (AI|AIMoveTo self "0, 0, 0" (Game|GetPlayerCharacter 0) 1.0 true
    (:OnSuccess
      _)
    (:OnFail
      _))
  (CallFunction|FollowPlayer))

(event Custom|Run%20Away
  (bind _returnvalue (Transformation|GetActorLocation))
  (bind _returnvalue_2 (Game|GetPlayerCharacter 0))
  (bind _returnvalue_3 (Transformation|GetActorLocation _returnvalue_2))
  (bind _returnvalue_4 (Math|Rotator|FindLookatRotation _returnvalue _returnvalue_3))
  (bind _returnvalue_5 (Math|Vector|GetForwardVector _returnvalue_4))
  (bind _returnvalue_6 (* _returnvalue_5 -5e+02))
  (bind _returnvalue_7 (+ _returnvalue _returnvalue_6))
  (bind (_x _y) (Math|Vector|BreakVector _returnvalue_7))
  (Development|PrintString "Run")
  (AI|AIMoveTo self (Math|Vector|MakeVector _x _y (.Z (Math|Vector|BreakVector _returnvalue))) 0 1.0 true
    (:OnSuccess
      _)
    (:OnFail
      _))
  (Utilities|FlowControl|Delay 2.0)
  (CallFunction|FollowPlayer))

(event Custom|Wait
  (Development|PrintString "wait")
  (Transformation|SetWorldRotation (Variables|Collision|GetCapsuleComponent) (Math|Rotator|MakeRotator 0.0 0.0 (+ (.Yaw (Math|Rotator|BreakRotator (Math|Conversions|RotationFromXVector (Math|Rotator|GetRotationXVector (Transformation|GetActorRotation (Game|GetPlayerCameraManager 0)))))) 1.8e+02)) false false))

(event EventBeginPlay
  (CallFunction|Wait)
  (bind _asbp_first_person_character (Utilities|Casting|CastToBP_FirstPersonCharacter (Game|GetPlayerCharacter 0)))
  (Variables|Default|SetHealth (Variables|/Game/FirstPerson/Blueprints/BP_FirstPersonCharacter.BP_FirstPersonCharacter_C|GetHealth _asbp_first_person_character)))

(event EventTick
  (params (DeltaSeconds :type Float%20%28single-precision%29))
  (CallFunction|Wait))

(fn ConstructionScript)